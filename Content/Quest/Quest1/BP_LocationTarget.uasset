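; BP_LocationTarget is a quest trigger volume that marks a location objective as reached when the third-person character overlaps it.
; On overlap it fires the character's objective event with its ObjectiveID, passes an XP reward to the player's exp message and shows a WBP_Location widget with LocationName.
; CompletedQuest reads that reward from the first stage of a hardcoded DT_Quest row.
; BeginPlay draws a temporary debug box around the trigger.
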(event `self.ReceiveBeginPlay`
  (bind _box (`self.Box`))
  (`KismetSystemLibrary.DrawDebugBox` (`PrimitiveComponent.GetCenterOfMass` _box "None") (`BoxComponent.GetScaledBoxExtent` _box) (struct :`R` 1.0 :`G` 0.091657 :`B` 0.341801 :`A` 1.0) (struct) 20.0 1.0))

(event `self.ReceiveActorBeginOverlap`
  (params (OtherActor :type "Actor Object Reference"))
  (bind _asbp_third_person_character (cast `/Game/Framework/Pawn/BP_ThirdPersonCharacter` OtherActor))
  (`/Game/Framework/Pawn/BP_ThirdPersonCharacter.OnObjectiveIDCaleedEvent` _asbp_third_person_character (`self.ObjectiveID`) 0)
  (bind _output_get (`self.CompletedQuest` true))
  (bind _newquantity (message `/Game/ThirdPerson/Interfaces/Food/BPI_Exp.AddExp` (`/Game/BFL_Utils.GetMyPlayerCharacter`) _output_get))
  (set `self.XPReward` _newquantity)
  (bind _returnvalue (`|CreateWidget` "/Game/Quest/WBP_Location.WBP_Location_C" null (`self.LocationName`)))
  (`UserWidget.AddToViewport` _returnvalue 0))

(fn `CompletedQuest`
  (params (CompletedQuest :type Boolean))
  (returns (Output_Get :type Integer))
  (bind _returnvalue (`|GetDataTableRow` "/Game/Quest/DT_Quest.DT_Quest" "10001")
    (:`then`
      (for _array_element (`.Stages_16_82C4C0FA4FF96654B6BC7DA836C951E1` (break `/Game/Quest/S_QuestDetails` _returnvalue))
        (bind _output_get (set `self.XPReward` (`KismetMathLibrary.SelectInt` (`.XPReward_9_110B0BF44FF87A026DA431ABD93F1642` (break `/Game/Quest/S_StageDetails` _array_element)) 0 CompletedQuest)))
        (return _output_get)))))

(fn `UserConstructionScript`)