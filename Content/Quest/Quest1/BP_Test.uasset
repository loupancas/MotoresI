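; BP_Test is a quest pickup actor, apparently for testing, that a BP_ThirdPersonCharacter collects by overlapping it.
; On overlap it adds its item and quantity to the character's ACInventory, passes the quantity and quest index to that component's Quest function, then destroys itself.
; Its own Quest function reads the first stage's XPReward from one of two DT_Quest rows, but the result only feeds a disconnected debug print.
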(event `self.ReceiveActorBeginOverlap`
  (params (OtherActor :type "Actor Object Reference"))
  (bind _index (`self.Index`))
  (bind _asbp_third_person_character (cast `/Game/Framework/Pawn/BP_ThirdPersonCharacter` OtherActor))
  (bind _ac_inventory (`/Game/Framework/Pawn/BP_ThirdPersonCharacter.AC_Inventory` _asbp_third_person_character))
  (`/Game/Quest/AC_Inventory.AddToInventory` _ac_inventory (`self.Item`) (`self.AddedQuantity`))
  (bind _xprewards (`self. Quest` _index))
  (`/Game/Quest/AC_Inventory.Quest` _ac_inventory (`self.AddedQuantity`) _index)
  (`self.K2_DestroyActor`))

(fn ` Quest`
  (params (Index :type Integer))
  (returns (XPRewards :type Integer))
  (bind _returnvalue (`|GetDataTableRow` "/Game/Quest/DT_Quest.DT_Quest" (select `int` Index :`0` "10001" :`1` "10002" :!type "Name"))
    (:`then`
      (for _array_element (`.Stages_16_82C4C0FA4FF96654B6BC7DA836C951E1` (break `/Game/Quest/S_QuestDetails` _returnvalue))
        (bind _output_get (set `self.XPReward` (`.XPReward_9_110B0BF44FF87A026DA431ABD93F1642` (break `/Game/Quest/S_StageDetails` _array_element))))
        (return _output_get)))))

(fn `UserConstructionScript`)