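; Interactable NPC for Quest1 that awards quest XP to the player and reports its objective ID.
; InteractWith prints ObjectiveID, calls CompletedQuest, passes the result to the player character's AddExpMessage, then returns the ID.
; CompletedQuest reads a hardcoded DT_Quest row and returns from inside the Stages loop, so only the first stage's XP counts.
; Interaction getters return fixed values with an empty prompt, and Lookat is empty.
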(event `self.ReceiveBeginPlay`)

(event `/Game/ThirdPerson/Interfaces/BPI_QuestInteraction.LookAt`)

(fn `CompletedQuest`
  (params (Completed :type Boolean))
  (returns (Output_Get :type Integer))
  (bind _returnvalue (`|GetDataTableRow` "/Game/Quest/DT_Quest.DT_Quest" "10001")
    (:`then`
      (for _array_element (`.Stages_16_82C4C0FA4FF96654B6BC7DA836C951E1` (break `/Game/Quest/S_QuestDetails` _returnvalue))
        (bind _output_get (set `self.XPReward` (`KismetMathLibrary.SelectInt` (`.XPReward_9_110B0BF44FF87A026DA431ABD93F1642` (break `/Game/Quest/S_StageDetails` _array_element)) 0 Completed)))
        (return _output_get)))))

(fn `GetHoldDuration`
  (returns (duration :type "Float (double-precision)"))
  (return 0.0))

(fn `GetInteractionLocation`
  (returns (Location :type "Vector Structure"))
  (return (0.0 0.0 0.0)))

(fn `GetInteractionType`
  (returns (Type :type "/Game/ThirdPerson/Interfaces/E_Interaction Enum"))
  (return "NewEnumerator2"))

(fn `GetTapCount`
  (returns (count :type Integer))
  (return 2))

(fn `InteractionPrompt`
  (returns (Value :type Text))
  (return ""))

(fn `InteractWith`
  (returns (ObjectiveID :type String))
  (bind _objective_id (`self.Objective ID`))
  (`KismetSystemLibrary.PrintString` _objective_id)
  (bind _output_get (`self.CompletedQuest` true))
  (bind _newquantity (message `/Game/ThirdPerson/Interfaces/Food/BPI_Exp.AddExp` (`/Game/BFL_Utils.GetMyPlayerCharacter`) _output_get))
  (set `self.XPReward` _newquantity)
  (return _objective_id))

(fn `UserConstructionScript`)