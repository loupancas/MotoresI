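; Quest log component that records active and completed quest IDs and spawns a Quest_Base actor for each new quest.
; Completion moves the ID to the completed list, sets TurnOn on the matching actor and calls OnQuestCompleted.
; Turn-in only prints the current stage's XP reward before completing the quest.
; Tracking creates one WBP_QuestTracker widget, then reuses it through Update.
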(fn `AddNewQuest`
  (params (QuestID :type Name))
  (returns (ReturnValue :type "/Game/Quest/Quest_Base Object Reference"))
  (`KismetArrayLibrary.Array_AddUnique` (`self.CurrentActiveQuests`) QuestID)
  (bind _returnvalue (`|SpawnActorFromClass` "/Game/Quest/Quest_Base.Quest_Base_C" (`KismetMathLibrary.MakeTransform` (0.0 0.0 0.0)) "Undefined" "MultiplyWithRoot" null QuestID null))
  (`KismetArrayLibrary.Array_Add` (`self.CurrentQuest`) _returnvalue)
  (return _returnvalue))

(fn `CompletedQuests`
  (params (QuestID :type "Name (by ref)"))
  (`KismetArrayLibrary.Array_AddUnique` (`self.CompletedQuest`) QuestID)
  (`KismetArrayLibrary.Array_RemoveItem` (`self.CurrentActiveQuests`) QuestID)
  (bind _array_element (`self.GetQuestActor` QuestID))
  (set `/Game/Quest/Quest_Base.TurnOn` true _array_element)
  (`self.OnQuestCompleted` _array_element))

(fn `GetQuestActor`
  (params (QuestID :type Name))
  (returns (`Array Element` :type "/Game/Quest/Quest_Base Object Reference"))
  (for _array_element (`self.CurrentQuest`)
    (if (== (`/Game/Quest/Quest_Base.QuestID` _array_element) QuestID)
      (return _array_element))))

(fn `QueryActiveQuest`
  (params (QuestID :type Name))
  (returns (ReturnValue :type Boolean))
  (return (`KismetArrayLibrary.Array_Contains` (`self.CurrentActiveQuests`) QuestID)))

(fn `QueryCompletedQuest`
  (params (QuestID :type Name))
  (returns (ReturnValue :type Boolean) (TurnOn :type Boolean))
  (bind _returnvalue (`KismetArrayLibrary.Array_Contains` (`self.CompletedQuest`) QuestID))
  (bind _array_element (`self.GetQuestActor` QuestID))
  (`/Engine/EditorBlueprintResources/StandardMacros.IsValid` _array_element
    (:`Is Valid`
      (return _returnvalue (`/Game/Quest/Quest_Base.TurnOn` _array_element)))
    (:`Is Not Valid`
      (return _returnvalue true))))

(fn `TrackQuest`
  (params (QuestActor :type "/Game/Quest/Quest_Base Object Reference"))
  (bind _tracker (`self.Tracker`)
    (:`then`
      (`/Game/Quest/WBP_QuestTracker.Update` _tracker QuestActor))
    (:`else`
      (bind _returnvalue (`|CreateWidget` "/Game/Quest/WBP_QuestTracker.WBP_QuestTracker_C" null QuestActor))
      (bind _output_get (set `self.Tracker` _returnvalue))
      (`UserWidget.AddToViewport` _output_get -1))))

(fn `TurnInQuest`
  (params (QuestID :type Name))
  (`|ExecutionSequence`
    (:`then_0`
      (bind _array_element (`self.GetQuestActor` QuestID))
      (`KismetSystemLibrary.PrintString` (`KismetTextLibrary.Conv_TextToString` (`|FormatText` "XP {XP}" (`.XPReward_9_110B0BF44FF87A026DA431ABD93F1642` (break `/Game/Quest/S_StageDetails` (`/Game/Quest/Quest_Base.CurrentStageDetails` _array_element)))))))
    (:`then_1`
      (`self.CompletedQuests` QuestID))))