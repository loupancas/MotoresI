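; Quest-giver NPC actor that the player can interact with through a set of interaction functions.
; InteractWith forwards to the quest giver component, prints the result as apparent debug output and returns it.
; The interaction queries report the Scene component's location and the Type and Count variables, with zero hold duration and an empty prompt.
; The event graph and construction script contain no logic.
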(fn `GetHoldDuration`
  (returns (duration :type "Float (double-precision)"))
  (return 0.0))

(fn `GetInteractionLocation`
  (returns (Location :type "Vector Structure"))
  (return (`SceneComponent.K2_GetComponentLocation` (`self.Scene`))))

(fn `GetInteractionType`
  (returns (Type :type "/Game/ThirdPerson/Interfaces/E_Interaction Enum"))
  (return (`self.Type`)))

(fn `GetTapCount`
  (returns (count :type Integer))
  (return (`self.Count`)))

(fn `InteractionPrompt`
  (returns (Value :type Text))
  (return ""))

(fn `InteractWith`
  (returns (ObjectiveID :type String))
  (bind _objectiveid (`/Game/ThirdPerson/Interfaces/BPI_QuestInteraction.InteractWith` (`self.AC_QuestGiverComponent`)))
  (`KismetSystemLibrary.PrintString` _objectiveid)
  (return _objectiveid))

(fn `UserConstructionScript`)