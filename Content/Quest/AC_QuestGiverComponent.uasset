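; Quest giver component that offers a quest to the player and presents its rewards on completion.
; InteractWith checks the player's quest log, then either auto-adds a new quest or opens the quest panel, according to its data table row.
; For a known quest it shows the rewards widget if completed and TurnOn is false.
; Handled interactions return the owner's display name; DisplayQuest reads QuestData's table, other lookups use DT_Quest directly.
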(fn `DisplayQuest`
  (bind (_questdata_datatable _questdata_rowname) (break `DataTableRowHandle` (`self.QuestData`)))
  (bind _returnvalue (`|GetDataTableRow` _questdata_datatable _questdata_rowname)
    (:`then`
      (bind _returnvalue_2 (`|CreateWidget` "/Game/Quest/WBP_QuestGiverPanel.WBP_QuestGiverPanel_C" null _returnvalue _questdata_rowname))
      (`UserWidget.AddToViewport` _returnvalue_2 0))))

(fn `DisplayRewards`
  (bind (_questdata_datatable _questdata_rowname) (break `DataTableRowHandle` (`self.QuestData`)))
  (bind _returnvalue (`|GetDataTableRow` "/Game/Quest/DT_Quest.DT_Quest" _questdata_rowname)
    (:`then`
      (bind _returnvalue_2 (`|CreateWidget` "/Game/Quest/WBP_Rewards.WBP_Rewards_C" null _returnvalue _questdata_rowname))
      (`UserWidget.AddToViewport` _returnvalue_2 0))))

(fn `InteractWith`
  (returns (ObjectiveID :type String))
  (bind (_questdata_datatable _questdata_rowname) (break `DataTableRowHandle` (`self.QuestData`)))
  (bind (_questdata_datatable_2 _questdata_rowname_2) (break `DataTableRowHandle` (`self.QuestData`)))
  (bind (_questdata_datatable_3 _questdata_rowname_3) (break `DataTableRowHandle` (`self.QuestData`)))
  (bind (_questdata_datatable_4 _questdata_rowname_4) (break `DataTableRowHandle` (`self.QuestData`)))
  (bind _returnvalue (`Actor.GetComponentByClass` (`GameplayStatics.GetPlayerCharacter` 0) "/Game/Quest/AC_QuestLogComponent.AC_QuestLogComponent_C"))
  (bind _returnvalue_2 (`KismetSystemLibrary.GetDisplayName` (`self.GetOwner`)))
  (bind _ac_quest (`/Game/Framework/Pawn/BP_ThirdPersonCharacter.AC_Quest` (`/Game/BFL_Utils.GetMyPlayerCharacter`)))
  (if (and (not (`/Game/Quest/AC_QuestLogComponent.QueryActiveQuest` _ac_quest _questdata_rowname_2)) (not (`/Game/Quest/AC_QuestLogComponent.QueryCompletedQuest` _ac_quest _questdata_rowname_2)))
    (bind _returnvalue_3 (`|GetDataTableRow` "/Game/Quest/DT_Quest.DT_Quest" _questdata_rowname_4)
      (:`then`
        (if (`.AutoAcepted_20_CF8EE93D4160386E2C97DA8D52DE9625` (break `/Game/Quest/S_QuestDetails` _returnvalue_3))
          (`/Engine/EditorBlueprintResources/StandardMacros.IsValid` _returnvalue
            (:`Is Valid`
              (`/Game/Quest/AC_QuestLogComponent.AddNewQuest` _returnvalue _questdata_rowname_3)
              (return (`KismetSystemLibrary.GetDisplayName` (`self.GetOwner`)))))
          (else
            (`self.DisplayQuest`)
            (return _returnvalue_2)))))
    (else
      (`KismetSystemLibrary.PrintString` "Alredy on Quest")
      (bind _array_element (`/Game/Quest/AC_QuestLogComponent.GetQuestActor` (`/Game/Framework/Pawn/BP_ThirdPersonCharacter.AC_Quest` (`/Game/BFL_Utils.GetMyPlayerCharacter`)) _questdata_rowname))
      (if (and (`/Game/Quest/Quest_Base.IsCompleted` _array_element) (not (`/Game/Quest/Quest_Base.TurnOn` _array_element)))
        (`self.DisplayRewards`)
        (return _returnvalue_2)))))