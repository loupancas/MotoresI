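; BP_Test_Child is a test child Blueprint of a quest item pickup that a player collects by walking into it.
; On overlap with BP_ThirdPersonCharacter, it adds Item and AddedQuantity to ACInventory, passes the quantity and Index to that component's Quest function, then destroys itself.
; Its Quest override only forwards to the parent.
; The parent overlap call and debug print are disconnected.
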(event `self.ReceiveActorBeginOverlap`
  (params (OtherActor :type "Actor Object Reference"))
  (bind _index (`self.Index`))
  (bind _asbp_third_person_character (cast `/Game/Framework/Pawn/BP_ThirdPersonCharacter` OtherActor))
  (bind _ac_inventory (`/Game/Framework/Pawn/BP_ThirdPersonCharacter.AC_Inventory` _asbp_third_person_character))
  (`/Game/Quest/AC_Inventory.AddToInventory` _ac_inventory (`self.Item`) (`self.AddedQuantity`))
  (bind _xprewards (`self. Quest` _index))
  (`/Game/Quest/AC_Inventory.Quest` _ac_inventory (`self.AddedQuantity`) _index)
  (`self.K2_DestroyActor`))

(fn ` Quest`
  (params (Index :type Integer))
  (returns (XPRewards :type Integer))
  (bind _xprewards (`parent. Quest` Index))
  (return _xprewards))

(fn `UserConstructionScript`
  (`parent.UserConstructionScript`))