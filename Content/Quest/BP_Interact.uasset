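; BP_Interact is a quest object that reports objective progress when a BP_ThirdPersonCharacter overlaps it.
; On overlap it calls InteractWith on the character, not itself, and passes the result as ObjectiveID with value 1 to the character's CallOnObjectiveIDCaleedEvent.
; Its own InteractWith prints and returns "strangeobject".
; The other interaction functions (prompt, type, location, hold duration, tap count) return only placeholder defaults.
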(event `self.ReceiveActorBeginOverlap`
  (params (OtherActor :type "Actor Object Reference"))
  (bind _asbp_third_person_character (cast `/Game/Framework/Pawn/BP_ThirdPersonCharacter` OtherActor))
  (bind _objectiveid (`/Game/Framework/Pawn/BP_ThirdPersonCharacter.InteractWith` _asbp_third_person_character))
  (`/Game/Framework/Pawn/BP_ThirdPersonCharacter.OnObjectiveIDCaleedEvent` _asbp_third_person_character _objectiveid 1))

(fn `GetHoldDuration`
  (returns (duration :type "Float (double-precision)"))
  (return 0.0))

(fn `GetInteractionLocation`
  (returns (Location :type "Vector Structure"))
  (return (0.0 0.0 0.0)))

(fn `GetInteractionType`
  (returns (Type :type "/Game/ThirdPerson/Interfaces/E_Interaction Enum"))
  (return "NewEnumerator0"))

(fn `GetTapCount`
  (returns (count :type Integer))
  (return 0))

(fn `InteractionPrompt`
  (returns (Value :type Text))
  (return ""))

(fn `InteractWith`
  (returns (ObjectiveID :type String))
  (`KismetSystemLibrary.PrintString` "strangeobject")
  (return "strangeobject"))

(fn `UserConstructionScript`)