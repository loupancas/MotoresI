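; BP_NPC_Interact is a quest NPC actor with interaction handlers that are mostly stubs.
; InteractWith prints and returns its ObjectiveID, while the other getters return fixed or empty defaults for type, tap count, hold duration, location and prompt.
; Lookat and Interact are empty, and the logic reporting the ObjectiveID to the player's PlayerInteractorComponent is disconnected, so it never runs.
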(event `self.ReceiveBeginPlay`)

(event `/Game/ThirdPerson/Interfaces/BPI_QuestInteraction.LookAt`)

(event `/Game/ThirdPerson/Interfaces/BPI_Interactable.Interact`
  (params (Interactor :type "Actor Object Reference")))

(fn `GetHoldDuration`
  (returns (duration :type "Float (double-precision)"))
  (return 0.0))

(fn `GetInteractionLocation`
  (returns (Location :type "Vector Structure"))
  (return (0.0 0.0 0.0)))

(fn `GetInteractionType`
  (returns (Type :type "/Game/ThirdPerson/Interfaces/E_Interaction Enum"))
  (return "NewEnumerator2"))

(fn `GetTapCount`
  (returns (count :type Integer))
  (return 2))

(fn `InteractionPrompt`
  (returns (Value :type Text))
  (return ""))

(fn `InteractWith`
  (returns (ObjectiveID :type String))
  (bind _objective_id (`self.Objective ID`))
  (`KismetSystemLibrary.PrintString` _objective_id)
  (return _objective_id))

(fn `UserConstructionScript`)