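; Game instance that handles level travel, completed-level progress, saving and sound playback for the TD game.
; Completing a level records its index and writes it with the player's data to a BP_TD_SaveGame slot.
; Menu loading reads that slot, sets a load flag and opens the saved level, while a separate LoadGame function restores player data and progress.
; PlaySound looks up 2D sounds by name, falling back to an ambient sound.
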(event `self.ReceiveInit`
  (`parent.ReceiveInit`))

(event `MenuLoadGame`
  (bind _returnvalue (`GameplayStatics.GetPlayerController` 0))
  (set `self.LoagGame` true)
  (bind _saveslot (`self.Game Load`))
  (`GameplayStatics.OpenLevel` (`KismetStringLibrary.Conv_StringToName` _saveslot))
  (set `PlayerController.bShowMouseCursor` false _returnvalue)
  (`WidgetBlueprintLibrary.SetInputMode_GameOnly` _returnvalue))

(fn `DefaultValues`
  (params (PlayerData :type "/Game/Framework/SaveSystem/S_GameSave Structure"))
  (locals (NewLocalVar :type "/Game/ThirdPerson/Interfaces/Weapons/BP_WeaponMaster Class Reference") (NewLocalVar_0 :type "/Game/ThirdPerson/Interfaces/Weapons/BP_WeaponMaster Class Reference") (NewLocalVar_1 :type "Float (double-precision)") (NewLocalVar_2 :type "Transform Structure") (NewLocalVar_3 :type Integer) (NewLocalVar_4 :type "Rotator Structure"))
  (bind (_transform _arc _playerhealth _controlerdirection _food _axe) (break `/Game/Framework/SaveSystem/S_GameSave` PlayerData))
  (set `local.NewLocalVar_2` _transform)
  (set `local.NewLocalVar_0` _arc)
  (set `local.NewLocalVar_1` _playerhealth)
  (set `local.NewLocalVar_4` _controlerdirection)
  (set `local.NewLocalVar_3` _food)
  (set `local.NewLocalVar` _axe)
  (return))

(fn `Game Load`
  (returns (SaveSlot :type String))
  (`KismetArrayLibrary.Array_Clear` (`self.Completed Levels`))
  (bind _returnvalue (`GameplayStatics.LoadGameFromSlot` (`self.Slot Name`)))
  (bind _asbp_td_save_game (cast `/Game/BP_TD_SaveGame` _returnvalue))
  (bind _output_get (set `self.SaveRef` _asbp_td_save_game))
  (return (`/Game/BP_TD_SaveGame.SaveSlot` _output_get)))

(fn `GetGameData`
  (returns (GData :type "/Game/BP_TD_SaveGame Object Reference"))
  (return (`self.PlayerSaveData`)))

(fn `IsLevelCompleted`
  (params (TheIndex :type Integer))
  (returns (ReturnValue :type Boolean))
  (return (`KismetArrayLibrary.Array_Contains` (`self.Completed Levels`) TheIndex)))

(fn `LoadGame`
  (bind _saveref (`self.SaveRef`))
  (`/Game/Framework/Pawn/BP_ThirdPersonCharacter.UsePlayerSave` (`self.PlayerCharacter`) (`/Game/BP_TD_SaveGame.GameData` _saveref))
  (set `self.Completed Levels` (`/Game/BP_TD_SaveGame.CompletedLevels` _saveref)))

(fn `OnLevelCompleted`
  (`KismetArrayLibrary.Array_AddUnique` (`self.Completed Levels`) (`self.CurrentLvl`))
  (`self.Save Game`))

(fn `OnMainMenu`
  (`GameplayStatics.OpenLevelBySoftObjectPtr` "/Game/Menu/Menu.Menu"))

(fn `OnPlayLevel`
  (params (TheIndex :type Integer))
  (bind _output (`|GetArrayItem` (`self.levelNames`) (`local.TheIndex`)))
  (if (not (== _output "None"))
    (set `self.CurrentLvl` (`local.TheIndex`))
    (`GameplayStatics.OpenLevel` _output)))

(fn `PlaySound`
  (params (SoundName :type String))
  (locals (SoundBase :type "SoundBase Object Reference" :default "/Script/Engine.SoundCue'/Game/ThirdPerson/Blueprints/Sounds/AmbientSound.AmbientSound'"))
  (bind (_value _returnvalue) (`BlueprintMapLibrary.Map_Find` (`self.Sounds`) (`self.SoundName`)))
  (`|ExecutionSequence`
    (:`then_0`
      (if _returnvalue
        (set `local.SoundBase` _value)
        (else
          (set `local.SoundBase` "/Game/ThirdPerson/Blueprints/Sounds/AmbientSound.AmbientSound"))))
    (:`then_1`
      (bind _soundbase (`local.SoundBase`)
        (:`then`
          (`GameplayStatics.SpawnSound2D` _soundbase 1.0 1.0 0.0 null))
        (:`else`)))))

(fn `Save Game`
  (bind _returnvalue (`GameplayStatics.CreateSaveGameObject` "/Game/BP_TD_SaveGame.BP_TD_SaveGame_C"))
  (bind _output_get (set `self.SaveRef` _returnvalue))
  (set `/Game/BP_TD_SaveGame.CompletedLevels` (`self.Completed Levels`) _output_get)
  (bind _player_save (`/Game/Framework/Pawn/BP_ThirdPersonCharacter.GetPlayerSaveData` (`self.PlayerCharacter`)))
  (set `/Game/BP_TD_SaveGame.GameData` _player_save _output_get)
  (bind _returnvalue_2 (`GameplayStatics.SaveGameToSlot` _output_get (`self.Slot Name`)))
  (if (not _returnvalue_2)
    (`KismetSystemLibrary.PrintString` "failedsave")))