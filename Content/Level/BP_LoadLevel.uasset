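; Level transition trigger that opens the level named by LevelName when a BP_ThirdPersonCharacter overlaps its box.
; Compares the player's experience to NeededExp and prints "Falta Exp" when it falls short.
; The load sequence clears all widgets, shows WBP_LoadingGame and disables input for a short fixed delay before opening the level by name.
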(event `self.Box.OnComponentBeginOverlap`
  (params (OverlappedComponent :type "PrimitiveComponent Object Reference") (OtherActor :type "Actor Object Reference") (OtherComp :type "PrimitiveComponent Object Reference") (OtherBodyIndex :type Integer) (bFromSweep :type Boolean) (SweepResult :type "HitResult Structure (by ref)"))
  (bind _returnvalue (`GameplayStatics.GetPlayerController` 0))
  (cast `/Game/Framework/Pawn/BP_ThirdPersonCharacter` OtherActor)
  (bind _quantity (`/Game/Framework/Pawn/BP_ThirdPersonCharacter.GetExpQuantity` (`/Game/BFL_Utils.GetMyPlayerCharacter`)))
  (if (not (>= _quantity (`self.NeededExp`)))
    (`KismetSystemLibrary.PrintString` "Falta Exp"))
  (`WidgetLayoutLibrary.RemoveAllWidgets`)
  (bind _returnvalue_2 (`|CreateWidget` "/Game/Framework/SaveSystem/WBP_LoadingGame.WBP_LoadingGame_C" _returnvalue))
  (`self.DisableInput` _returnvalue)
  (`UserWidget.AddToViewport` _returnvalue_2 0)
  (`KismetSystemLibrary.Delay` 1.0)
  (`self.EnableInput` _returnvalue)
  (`GameplayStatics.OpenLevel` (`self.Level Name`)))

(fn `UserConstructionScript`)