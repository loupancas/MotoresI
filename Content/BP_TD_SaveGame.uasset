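; BP_TD_SaveGame is a save game object that stores and restores the player's quest state.
; It copies active and completed quest lists from a quest log, and records each quest's stage and objective progress in a map keyed by quest ID.
; Loading re-adds each active quest to the quest component, reapplies its saved stage and progress, then restores both lists.
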(fn `LoadQuests`
  (params (QuestComponent :type "/Game/Quest/AC_Quest Object Reference"))
  (for _array_element (`self.CurrentActiveQuests`)
    (bind _returnvalue (`/Game/Quest/AC_Quest.AddNewQuest` QuestComponent _array_element))
    (bind (_progress _currentstage) (break `/Game/Quest/S_SaveQuestData` (`BlueprintMapLibrary.Map_Find` (`self.QuestProgress`) _array_element)))
    (set `/Game/Quest/Quest_Base.CurrentStage` _currentstage _returnvalue)
    (set `/Game/Quest/Quest_Base.CurrentObjectivesProgress` _progress _returnvalue))
  (set `/Game/Quest/AC_Quest.CurrentActiveQuests` (`self.CurrentActiveQuests`) QuestComponent)
  (set `/Game/Quest/AC_Quest.CompletedQuest` (`self.CompleteQuests`) QuestComponent))

(fn `SaveQuestDetails`
  (params (Quest :type "/Game/Quest/Quest_Base Object Reference"))
  (`BlueprintMapLibrary.Map_Add` (`self.QuestProgress`) (`/Game/Quest/Quest_Base.QuetID` Quest) (make `/Game/Quest/S_SaveQuestData` (`/Game/Quest/Quest_Base.CurrentObjectivesProgress` Quest) (`/Game/Quest/Quest_Base.CurrentStage` Quest))))

(fn `SaveQustLog`
  (params (QuestLog :type "/Game/Quest/AC_Quest Object Reference"))
  (set `self.CurrentActiveQuests` (`/Game/Quest/AC_Quest.CurrentActiveQuests` QuestLog))
  (set `self.CompleteQuests` (`/Game/Quest/AC_Quest.CompletedQuest` QuestLog)))