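; Player controller for the main menu that shows the menu widget and opens its sub-screens.
; BeginPlay sets UI-only input, shows the cursor and adds WBP_MainMenu1 to the viewport.
; Separate functions add level select, settings, credits or save-slot widgets, tracked in WBPModel, which OnMainMenu removes and clears.
; OnSelectHowToPlay also opens WBP_Credits rather than a dedicated screen.
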(event `self.ReceiveBeginPlay`
  (`WidgetBlueprintLibrary.SetInputMode_UIOnlyEx` self null)
  (set `self.bShowMouseCursor` true)
  (bind _returnvalue (`|CreateWidget` "/Game/Framework/Menu/WBP_MainMenu1.WBP_MainMenu1_C"))
  (bind _output_get (set `self.MainMENU` _returnvalue))
  (`UserWidget.AddToViewport` _output_get 0))

(fn `On Save Game`
  (bind _returnvalue (`|CreateWidget` "/Game/WBP_SelectSaveSlot.WBP_SelectSaveSlot_C"))
  (bind _output_get (set `self.WBPModel` _returnvalue))
  (`UserWidget.AddToViewport` _output_get 0))

(fn `On Select Credits`
  (bind _returnvalue (`|CreateWidget` "/Game/Framework/Menu/WBP_Credits.WBP_Credits_C"))
  (bind _output_get (set `self.WBPModel` _returnvalue))
  (`UserWidget.AddToViewport` _output_get 0))

(fn `On Select HowToPlay`
  (bind _returnvalue (`|CreateWidget` "/Game/Framework/Menu/WBP_Credits.WBP_Credits_C"))
  (bind _output_get (set `self.WBPModel` _returnvalue))
  (`UserWidget.AddToViewport` _output_get 0))

(fn `On Select Lvl Slot`
  (bind _returnvalue (`|CreateWidget` "/Game/WBP_LvlSelect.WBP_LvlSelect_C"))
  (bind _output_get (set `self.WBPModel` _returnvalue))
  (`UserWidget.AddToViewport` _output_get 0))

(fn `On Select Settings`
  (bind _returnvalue (`|CreateWidget` "/Game/Framework/Menu/WBP_Settings.WBP_Settings_C"))
  (bind _output_get (set `self.WBPModel` _returnvalue))
  (`UserWidget.AddToViewport` _output_get 0))

(fn `OnMainMenu`
  (bind _wbpmodel (`self.WBPModel`)
    (:`then`
      (`Widget.RemoveFromParent` _wbpmodel)
      (set `self.WBPModel` null))
    (:`else`)))

(fn `UserConstructionScript`)